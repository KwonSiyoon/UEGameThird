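; Bear monster character that spots and chases the player warrior, driven by a state enum mirrored to its AI Blackboard.
; Pawn sensing sets the Chase state, target and walk speed, while Tick drops the chase once the target leaves sight radius.
; Actor overlaps play a timeline that drives a hit value on its dynamic stone material.
; Locomotion, attack and death handlers are empty stubs, and the camera shake is unwired.
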(event `self.ReceiveBeginPlay`
  (bind _returnvalue (`PrimitiveComponent.CreateDynamicMaterialInstance` (`self.Mesh`) 0 "/Game/InfinityBladeAdversaries/Enemy/Enemy_Bear/Materials/M_Bear_Stone_Inst.M_Bear_Stone_Inst" "None"))
  (set `self.DynamicInstance` _returnvalue))

(event `self.ReceiveActorBeginOverlap`
  (params (OtherActor :type "Actor Object Reference"))
  (bind (_direction _effectvalue) (`Timeline|HitEffect` :!via `PlayFromStart`)
    (:`Update`
      (`MaterialInstanceDynamic.SetScalarParameterValue` (`self.DynamicInstance`) "HitValue" _effectvalue))))

(event `SetState`
  (params (NewState :type "/Game/Blueprints/Monster/E_BearState Enum" :default "NewEnumerator0"))
  (if (`|EnumInequality` (`self.State`) "NewEnumerator3")
    (if (`|EnumInequality` (`self.State`) NewState)
      (bind _output_get (set `self.State` NewState))
      (`BlackboardComponent.SetValueAsEnum` (`AIBlueprintHelperLibrary.GetBlackboard` (`AIBlueprintHelperLibrary.GetAIController` self)) (`self.StateKey`) _output_get))))

(event `self.PawnSensing.OnSeePawn`
  (params (Pawn :type "Pawn Object Reference"))
  (if (`|EnumEquality` (`self.State`) "NewEnumerator0")
    (bind _asbp_warrior (cast `/Game/Blueprints/Warrior/BP_Warrior` Pawn))
    (if (`|EnumInequality` (`/Game/Blueprints/Warrior/BP_Warrior.State` _asbp_warrior) "NewEnumerator2")
      (`self.SetState` "NewEnumerator1")
      (bind _output_get (set `self.Instigator` Pawn))
      (`BlackboardComponent.SetValueAsObject` (`AIBlueprintHelperLibrary.GetBlackboard` null) (`self.TargetKey`) _output_get)
      (`|ExecutionSequence`
        (:`then_0`
          (switch `/Game/Blueprints/Monster/E_BearState` (`self.State`)
            (:`NewEnumerator0`
              (set `CharacterMovementComponent.MaxWalkSpeed` 200.0 (`self.CharacterMovement`)))
            (:`NewEnumerator1`
              (set `CharacterMovementComponent.MaxWalkSpeed` 500.0 (`self.CharacterMovement`)))
            (:`NewEnumerator2`
              (set `CharacterMovementComponent.MaxWalkSpeed` 0.0 (`self.CharacterMovement`) :!label _label))
            (:`NewEnumerator3`
              (goto _label))))))))

(event `self.ReceiveTick`
  (params (DeltaSeconds :type "Float (single-precision)"))
  (switch `/Game/Blueprints/Monster/E_BearState` (`self.State`)
    (:`NewEnumerator0`
      (`self.OnLocomotion`))
    (:`NewEnumerator1`
      (`self.OnChase`))
    (:`NewEnumerator2`
      (`self.OnAttack`))))

(event `OnLocomotion`)

(event `OnChase`
  (bind _instigator (`self.Instigator`))
  (`/Engine/EditorBlueprintResources/StandardMacros.IsValid` _instigator
    (:`Is Valid`
      (if (> (`KismetMathLibrary.Vector_Distance` (`self.K2_GetActorLocation` _instigator) (`self.K2_GetActorLocation`)) (`PawnSensingComponent.SightRadius` (`self.PawnSensing`)))
        (set `self.Instigator` null)
        (`self.SetState` "NewEnumerator0")))))

(event `OnAttack`)

(event `OnDead`)

(fn `UserConstructionScript`)
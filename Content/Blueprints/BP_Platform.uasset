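; BP_Platform is a moving platform actor that travels along the forward direction of its Arrow component.
; On BeginPlay it stores its starting location and plays the Move timeline.
; Each timeline update sets the location to that origin plus the Arrow's forward vector scaled by Alpha and MoveLength, without sweeping.
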(event `self.ReceiveBeginPlay`
  (set `self.OriginLocation` (`self.K2_GetActorLocation`))
  (bind (_direction _alpha) (`Timeline|Move`)
    (:`Update`
      (`self.K2_SetActorLocation` (+ (`self.OriginLocation`) (* (* _alpha (`self.MoveLength`)) (`SceneComponent.GetForwardVector` (`self.Arrow`))))))))

(fn `UserConstructionScript`)